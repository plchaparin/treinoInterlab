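; BP_piece1 is a game piece actor that moves and rotates in fixed steps when its custom events are called.
; MovaPeca and MovaPeca2 shift the root 100 units along negative and positive world X, while GiraPeca and GiraPeca2 apply opposite 90-degree turns.
; Each event is a single AddWorldTransform on DefaultSceneRoot, with no input handling, Tick logic or bounds checks in this Blueprint.
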(event `MovaPeca`
  (`SceneComponent.K2_AddWorldTransform` (`self.DefaultSceneRoot`) (`KismetMathLibrary.MakeTransform` (-100.0 0.0 0.0)) false false))

(event `GiraPeca2`
  (`SceneComponent.K2_AddWorldTransform` (`self.DefaultSceneRoot`) (`KismetMathLibrary.MakeTransform` (0.0 0.0 0.0) (struct :`Pitch` -90.0)) false false))

(event `MovaPeca2`
  (`SceneComponent.K2_AddWorldTransform` (`self.DefaultSceneRoot`) (`KismetMathLibrary.MakeTransform` (100.0 0.0 0.0)) false false))

(event `GiraPeca`
  (`SceneComponent.K2_AddWorldTransform` (`self.DefaultSceneRoot`) (`KismetMathLibrary.MakeTransform` (0.0 0.0 0.0) (struct :`Pitch` 90.0)) false false))

(fn `UserConstructionScript`)